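; BP_FlowTestHarness is a test actor for manually exercising the SimFlow system from the keyboard.
; On BeginPlay it adds a flow status widget to the viewport and, after a short delay, shows the mouse cursor.
; Number keys and F call SimFlow directly to start, restart, pause, retry, skip or fail tasks, send a Grab event, and quick save or load.
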(event EventBeginPlay
  (bind _returnvalue (UserInterface|CreateWidget "/Game/SimFlowTest/UI/WBP_FlowSatus.WBP_FlowSatus_C"))
  (UserInterface|Viewport|AddtoViewport _returnvalue 0)
  (Utilities|FlowControl|Delay 0.2)
  (Variables|/Script/Engine.PlayerController|SetbShowMouseCursor (Game|GetPlayerController 0) true))

(event Collision|EventActorBeginOverlap
  (params (OtherActor :type Actor%20Object%20Reference)))

(event EventTick
  (params (DeltaSeconds :type Float%20%28single-precision%29)))

(event Input|KeyboardEvents|8
  (params (Key :type Key%20Structure))
  (:Pressed
    (Class|SimFlowComponent|QuickLoad (Variables|Default|GetSimFlow))))

(event Input|KeyboardEvents|1
  (params (Key :type Key%20Structure))
  (:Pressed
    (Class|SimFlowComponent|StartFlow (Variables|Default|GetSimFlow))))

(event Input|KeyboardEvents|2
  (params (Key :type Key%20Structure))
  (:Pressed
    (Class|SimFlowComponent|RestartFlow (Variables|Default|GetSimFlow))))

(event Input|KeyboardEvents|3
  (params (Key :type Key%20Structure))
  (:Pressed
    (Class|SimFlowComponent|TogglePause (Variables|Default|GetSimFlow))))

(event Input|KeyboardEvents|4
  (params (Key :type Key%20Structure))
  (:Pressed
    (Class|SimFlowComponent|RetryCurrentTask (Variables|Default|GetSimFlow))))

(event Input|KeyboardEvents|5
  (params (Key :type Key%20Structure))
  (:Pressed
    (Class|SimFlowComponent|SkipCurrentTask (Variables|Default|GetSimFlow))))

(event Input|KeyboardEvents|F
  (params (Key :type Key%20Structure))
  (:Pressed
    (Class|SimFlowComponent|FailCurrentTask (Variables|Default|GetSimFlow))))

(event Input|KeyboardEvents|6
  (params (Key :type Key%20Structure))
  (:Pressed
    (Class|SimFlowComponent|SendEvent (Variables|Default|GetSimFlow) "(TagName=\"SimFlow.Event.Grab\")" 0)))

(event Input|KeyboardEvents|7
  (params (Key :type Key%20Structure))
  (:Pressed
    (Class|SimFlowComponent|QuickSave (Variables|Default|GetSimFlow))))

(fn ConstructionScript)